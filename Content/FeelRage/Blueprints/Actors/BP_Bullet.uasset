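; BP_Bullet is a projectile actor that damages enemies on hit and destroys itself on any collision.
; On BeginPlay it launches along the Character reference's forward vector at BulletSpeed.
; The sphere's hit event subtracts damage from the BP_Enemy's Health component.
; Enemies of type 2 take double damage from hits behind them, detected by a dot product of impact offset and enemy forward vector.
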(event `self.ReceiveBeginPlay`
  (set `MovementComponent.Velocity` (* (`self.GetActorForwardVector` (`self.Character`)) (`self.BulletSpeed`)) (`self.ProjectileMovement`)))

(event `self.Sphere.OnComponentHit`
  (params (HitComponent :type "PrimitiveComponent Object Reference") (OtherActor :type "Actor Object Reference") (OtherComp :type "PrimitiveComponent Object Reference") (NormalImpulse :type "Vector Structure") (Hit :type "HitResult Structure (by ref)"))
  (bind _asbp_enemy (cast `/Game/FeelRage/Characters/Enemy/BP/BP_Enemy` OtherActor)
    (:`then`
      (bind _output_get (set `self.BP_Enemy` _asbp_enemy))
      (if (== (`/Game/FeelRage/Characters/Enemy/BP/BP_Enemy.EnemyType` _output_get) 2)
        (if (< (`KismetMathLibrary.Dot_VectorVector` (- (`.ImpactPoint` (`GameplayStatics.BreakHitResult` Hit)) (`self.K2_GetActorLocation` (`self.BP_Enemy`))) (`self.GetActorForwardVector` (`self.BP_Enemy`))) 0.0)
          (`Health.SubtractHealth` (`/Game/FeelRage/Characters/Enemy/BP/BP_Enemy.Health` (`self.BP_Enemy`)) (* (`self.Damage`) 2))
          (`self.K2_DestroyActor`)
          (else
            (`Health.SubtractHealth` (`/Game/FeelRage/Characters/Enemy/BP/BP_Enemy.Health` (`self.BP_Enemy`)) (`self.Damage`))
            (`self.K2_DestroyActor`)))
        (else
          (`Health.SubtractHealth` (`/Game/FeelRage/Characters/Enemy/BP/BP_Enemy.Health` (`self.BP_Enemy`)) (`self.Damage`))
          (`self.K2_DestroyActor` :!label _label))))
    (:`CastFailed`
      (goto _label))))

(fn `UserConstructionScript`)