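; Ranged weapon actor that acts as a sniper or assault rifle, with stats set from its Weapons selection on BeginPlay.
; Attach disables the cube's collision and snaps the weapon to an actor's HandGrip_R socket.
; Attack spends ammo to spawn BP_Bullet ahead of the attacker, using a Gate and Delay to limit fire rate.
; A looping timer polls for an empty magazine and automatically refills it after the reload delay.
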(event `StartReloadTimer`
  ; RelaodCheck
  (bind _returnvalue (`KismetSystemLibrary.K2_SetTimerDelegate` (delegate `ReloadCheck`) 0.1 true :!label _label))
  (set `self.RelaodCheck` _returnvalue))

(event `self.ReceiveBeginPlay`
  ; SelectWeapon
  (switch `int` (`self.weapons`)
    (:`1`
      ;; SniperRifle
      (`self.Stats` 80 4500 3.0 5 1.0
        (:`Exit`
          _)))
    (:`2`
      ;; AssaultRifle
      (`self.Stats` 20 3000 2.0 30 0.1
        (:`Exit`
          _))))
  (set `self.CurrentAmmo` (`self.Ammo`))
  (goto _label))

(event `ReloadCheck`
  ; RelaodCheck
  (if (== (`self.CurrentAmmo`) 0)
    (`KismetSystemLibrary.K2_PauseTimerHandle` (`self.RelaodCheck`))
    (`KismetSystemLibrary.Delay` (`self.ReloadTime`))
    (set `self.CurrentAmmo` (`self.Ammo`))
    (`KismetSystemLibrary.K2_UnPauseTimerHandle` (`self.RelaodCheck`))
    (`self.StartReloadTimer`)))

(event `attach`
  (params (Actor :type "Actor Object Reference"))
  ; Attach
  (`PrimitiveComponent.SetCollisionEnabled` (`self.Cube`) "NoCollision")
  (`KismetSystemLibrary.Delay` 0.1)
  (`self.K2_AttachToActor` Actor "HandGrip_R" "SnapToTarget" "SnapToTarget" "KeepRelative"))

(event `Attack`
  (params (Actor :type "Actor Object Reference"))
  (bind _actor (`self.Actor`))
  ; Attack
  (set `self.Actor` Actor)
  (if (> (`self.CurrentAmmo`) 0)
    (`/Engine/EditorBlueprintResources/StandardMacros.Gate` false :!label _label_2
      (:`Exit`
        (`|ExecutionSequence`
          (:`then_0`
            (`/Engine/EditorBlueprintResources/StandardMacros.DecrementInt` (`self.CurrentAmmo`)
              (:`  `
                (`|SpawnActorFromClass` "/Game/FeelRage/Blueprints/Actors/BP_Bullet.BP_Bullet_C" (`KismetMathLibrary.Conv_VectorToTransform` (+ (`self.K2_GetActorLocation` _actor) (* (`self.GetActorForwardVector` _actor) 50))) "Undefined" "MultiplyWithRoot" null _actor (`self.SpeedOfBullet`) (`self.Damage`) null)
                (`KismetSystemLibrary.Delay` (`self.Fire Rate`))
                (goto _label_2 :!via `Open`))))
          (:`then_1`
            (goto _label_2 :!via `Close`)))))))

(fn `UserConstructionScript`)