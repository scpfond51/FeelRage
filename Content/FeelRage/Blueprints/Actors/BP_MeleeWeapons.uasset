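; Melee weapon actor that randomly becomes a knife, machete or "OgnedMachete" on BeginPlay, each setting damage, attack radius and reload time.
; Attach disables collision and snaps it to an actor's right-hand socket.
; Detach throws it along that actor's forward vector via ProjectileMovement, restoring collision after a short delay, with machetes overlapping pawns.
; Cube hits or overlaps subtract damage from BP_Enemy health.
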(event `self.ReceiveBeginPlay`
  (bind _output_get (set `self.Weapon` (`KismetMathLibrary.RandomIntegerInRange` 1 3)))
  (switch `int` _output_get
    (:`1`
      ; Knife
      (`self.Stats` 30 (2.35 2.35 2.0) 0.5))
    (:`2`
      ; Machete
      (`self.Stats` 30 (3.5 3.5 3.0) 0.8))
    (:`3`
      ; OgnedMachete
      (`self.Stats` 50 (3.5 3.5 3.0) 0.8))))

(event `attach`
  (params (Actor :type "Actor Object Reference"))
  (`PrimitiveComponent.SetCollisionEnabled` (`self.Cube`) "NoCollision")
  (`KismetSystemLibrary.Delay` 0.1)
  (`self.K2_AttachToActor` Actor "HandGrip_R" "SnapToTarget" "SnapToTarget" "KeepRelative"))

(event `Detach`
  (bind _cube (`self.Cube`))
  (bind _projectilemovement (`self.ProjectileMovement`))
  (`self.K2_DetachFromActor` "KeepWorld" "KeepWorld" "KeepWorld")
  (`|ExecutionSequence`
    (:`then_0`
      (`MovementComponent.SetUpdatedComponent` (`self.ProjectileMovement`) (`self.Cube`))
      (`ActorComponent.SetActive` _projectilemovement true false)
      (`ActorComponent.SetComponentTickEnabled` _projectilemovement true)
      (set `MovementComponent.Velocity` (* (`self.GetActorForwardVector` (stale `attach` Actor)) 1000) (`self.ProjectileMovement`)))
    (:`then_1`
      (`KismetSystemLibrary.Delay` 0.2)
      (switch `int` (`self.Weapon`)
        (:`1`
          (`PrimitiveComponent.SetCollisionEnabled` _cube "QueryAndPhysics"))
        (:`2`
          (`PrimitiveComponent.SetCollisionEnabled` _cube "QueryAndPhysics" :!label _label)
          (`PrimitiveComponent.SetCollisionResponseToChannel` (`self.Cube`) "ECC_Pawn" "ECR_Overlap"))
        (:`3`
          (goto _label))))))

(event `self.Cube.OnComponentHit`
  (params (HitComponent :type "PrimitiveComponent Object Reference") (OtherActor :type "Actor Object Reference") (OtherComp :type "PrimitiveComponent Object Reference") (NormalImpulse :type "Vector Structure") (Hit :type "HitResult Structure (by ref)"))
  (bind _asbp_enemy (cast `/Game/FeelRage/Characters/Enemy/BP_Enemy` OtherActor))
  (`Health.SubtractHealth` (`/Game/FeelRage/Characters/Enemy/BP_Enemy.Health` _asbp_enemy) (`self.Damage`)))

(event `self.Cube.OnComponentBeginOverlap`
  (params (OverlappedComponent :type "PrimitiveComponent Object Reference") (OtherActor :type "Actor Object Reference") (OtherComp :type "PrimitiveComponent Object Reference") (OtherBodyIndex :type Integer) (bFromSweep :type Boolean) (SweepResult :type "HitResult Structure (by ref)"))
  (bind _asbp_enemy (cast `/Game/FeelRage/Characters/Enemy/BP_Enemy` OtherActor))
  (`Health.SubtractHealth` (`/Game/FeelRage/Characters/Enemy/BP_Enemy.Health` _asbp_enemy) (`self.Damage`)))

(fn `UserConstructionScript`)