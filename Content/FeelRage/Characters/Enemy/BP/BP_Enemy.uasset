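; Enemy actor that randomly becomes a Flying or Fat chaser, unless preset as a two-phase Necromancer boss.
; A looping five-ray vision trace sets the player as target, which Tick turns toward to chase or, for the boss, to spawn more enemies.
; Capsule overlap gates a timed damage attack.
; Weapon and bullet hits turn it toward the player, trigger the boss's second phase at low health, and handle death.
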(event `TakedMeleeDamage`
  (bind _health (`Health.Health` (`self.Health`)))
  ; TakingDamage
  (`KismetSystemLibrary.PrintString` (`KismetStringLibrary.Conv_IntToString` _health) :!label _label)
  (`self.Hitted`)
  (`|ExecutionSequence`
    (:`then_0`
      (if (== (`self.EnemyType`) 3)
        (if (<= (`Health.Health` (`self.Health`)) 250)
          (`/Engine/EditorBlueprintResources/StandardMacros.DoOnce` false
            (:`Completed`
              (set `self.EnemyType` 4)
              ;; NegromantV2
              (`self.Stats` 20 250 (250.0 250.0 0.0) 3.0 2.0))))))
    (:`then_1`
      (if (<= _health 0)
        (if (== (`self.EnemyType`) 4)
          (`|ExecutionSequence`
            (:`then_0`
              (`KismetSystemLibrary.Delay` 3.0)
              (`GameplayStatics.OpenLevelBySoftObjectPtr` "/Game/FeelRage/Maps/L_Level1.L_Level1"))
            (:`then_1`
              (`/Game/ThirdPerson/Blueprints/BP_ThirdPersonCharacter.Kill` (`self.BP_ThirdPersonCharacter`) :!label _label_2)
              (`self.K2_DestroyActor`)))
          (else
            (goto _label_2)))))))

(event `self.ReceiveBeginPlay`
  ; Main
  ;; EventBeginPlay
  (bind _returnvalue (`GameplayStatics.GetActorOfClass` "/Game/ThirdPerson/Blueprints/BP_ThirdPersonCharacter.BP_ThirdPersonCharacter_C"))
  (set `self.BP_ThirdPersonCharacter` _returnvalue)
  (`self.CustomEvents`))

(event `self.CapsuleComponent.OnComponentHit`
  (params (HitComponent :type "PrimitiveComponent Object Reference") (OtherActor :type "Actor Object Reference") (OtherComp :type "PrimitiveComponent Object Reference") (NormalImpulse :type "Vector Structure") (Hit :type "HitResult Structure (by ref)"))
  ; TakingDamage
  (cast `/Game/FeelRage/Blueprints/Actors/BP_MeleeWeapons` OtherActor
    (:`then`
      (goto _label))
    (:`CastFailed`
      (cast `/Game/FeelRage/Blueprints/Actors/BP_Bullet` OtherActor)
      (goto _label))))

(event `CustomEvents`
  ; Main
  ;; CustomEvents
  (`self.SetEnemyType`)
  (`self.StartVision`)
  (`self.attacktimer`))

(event `StartVision`
  ; Vision
  (`KismetSystemLibrary.K2_SetTimerDelegate` (delegate `LineTraceVision`) 0.1 true))

(event `SetEnemyType`
  ; TypeSelection
  (if (!= (`self.EnemyType`) 3)
    (bind _output_get (set `self.EnemyType` (`KismetMathLibrary.RandomIntegerInRange` 1 2)))
    (switch `int` _output_get
      (:`1`
        ;; Flying
        (`self.Stats` 25 50 (600.0 600.0 0.0) 10.0))
      (:`2`
        ;; Fat
        (`self.Stats` 20 200 (250.0 250.0 0.0) 3.0)))
    (else
      ;; NegromantV1
      (`self.Stats` 0 500 (250.0 250.0 0.0) 3.0 5.0
        (:`exec`
          (`SkeletalMeshComponent.SetSkeletalMeshAsset` (`self.Mesh`) null))))))

(event `LineTraceVision`
  (bind _returnvalue (`self.K2_GetActorLocation`))
  (bind _returnvalue_2 (`self.K2_GetActorLocation`))
  (bind _returnvalue_3 (`self.K2_GetActorLocation`))
  (bind _returnvalue_4 (`self.K2_GetActorLocation`))
  (bind _returnvalue_5 (`self.K2_GetActorLocation`))
  ; Vision
  (`|ExecutionSequence`
    (:`then_0`
      (`self.LineTrace` _returnvalue_2 (+ (* (`self.GetActorForwardVector`) 1200) _returnvalue_2)))
    (:`then_1`
      (`self.LineTrace` _returnvalue_5 (+ (* (+ (`self.GetActorForwardVector`) (* (`self.GetActorRightVector`) 0.2)) 1000) _returnvalue_5)))
    (:`then_2`
      (`self.LineTrace` _returnvalue_4 (+ (* (- (`self.GetActorForwardVector`) (* (`self.GetActorRightVector`) 0.2)) 1000) _returnvalue_4)))
    (:`then_3`
      (`self.LineTrace` _returnvalue_3 (+ (* (+ (`self.GetActorForwardVector`) (* (`self.GetActorRightVector`) 0.5)) 800) _returnvalue_3)))
    (:`then_4`
      (`self.LineTrace` _returnvalue (+ (* (- (`self.GetActorForwardVector`) (* (`self.GetActorRightVector`) 0.5)) 800) _returnvalue)))))

(event `self.ReceiveTick`
  (params (DeltaSeconds :type "Float (single-precision)"))
  (bind _bp_target (`self.BP_Target`))
  ; Movements
  (if (not (`self.Attacking`))
    (if (`self.PlayerAtRage`)
      _
      (else
        _))
    (`/Engine/EditorBlueprintResources/StandardMacros.IsValid` _bp_target
      (:`Is Valid`
        (`self.K2_SetActorRotation` (* (`KismetMathLibrary.RInterpTo` (`self.K2_GetActorRotation`) (`KismetMathLibrary.MakeRotFromX` (- (`self.K2_GetActorLocation` _bp_target) (`self.K2_GetActorLocation`))) DeltaSeconds (`self.Rotation Speed`)) (100.0 100.0 0.0)))
        (switch `int` (`self.EnemyType`)
          (:`1`
            _)
          (:`2`
            _)
          (:`3`
            (`/Engine/EditorBlueprintResources/StandardMacros.DoOnce` false :!label _label_3
              (:`Completed`
                (`|ExecutionSequence`
                  (:`then_0`
                    (`self.Spawner` (`self.Spawner2`))
                    (goto _label_3 :!via `Reset`))
                  (:`then_1`
                    (`self.Spawner` (`self.Spawner1`))
                    (goto _label_3 :!via `Reset`))))))
          (:`4`
            (`|ExecutionSequence`
              (:`then_0`
                (goto _label_3))
              (:`then_1`
                _))))
        (`self.K2_AddActorWorldOffset` (* (`self.GetActorForwardVector`) (`self.Speed`) DeltaSeconds))))))

(event `Hitted`
  ; Movements
  (`self.K2_SetActorRotation` (* (`KismetMathLibrary.MakeRotFromX` (- (`self.K2_GetActorLocation` (`self.BP_ThirdPersonCharacter`)) (`self.K2_GetActorLocation`))) (100.0 100.0 0.0))))

(event `TurnBack`
  ; Movements
  (`self.K2_SetActorRotation` (`KismetMathLibrary.MakeRotator` (.roll (`self.K2_GetActorRotation`)) (.pitch (`self.K2_GetActorRotation`)) (+ (.yaw (`self.K2_GetActorRotation`)) 90.0))))

(event `attacktimer`
  ; Attack
  (`KismetSystemLibrary.K2_SetTimerDelegate` (delegate `Attack`) 1.0 true))

(event `Attack`
  ; Attack
  (`/Engine/EditorBlueprintResources/StandardMacros.Gate` true :!label _label_4
    (:`Exit`
      (bind _health (`/Game/ThirdPerson/Blueprints/BP_ThirdPersonCharacter.Health` (stale `self.Capsule.OnComponentBeginOverlap` _asbp_third_person_character)))
      (`Health.SubtractHealth` _health (`self.Damage`))
      (if (<= (`Health.Health` _health) 0)
        (`GameplayStatics.OpenLevelBySoftObjectPtr` "/Game/FeelRage/Maps/L_Level1.L_Level1")))))

(event `self.Capsule.OnComponentBeginOverlap`
  (params (OverlappedComponent :type "PrimitiveComponent Object Reference") (OtherActor :type "Actor Object Reference") (OtherComp :type "PrimitiveComponent Object Reference") (OtherBodyIndex :type Integer) (bFromSweep :type Boolean) (SweepResult :type "HitResult Structure (by ref)"))
  ; Attack
  (bind _asbp_third_person_character (cast `/Game/ThirdPerson/Blueprints/BP_ThirdPersonCharacter` OtherActor))
  (set `self.Attacking` true)
  (goto _label_4 :!via `Open`))

(event `self.Capsule.OnComponentEndOverlap`
  (params (OverlappedComponent :type "PrimitiveComponent Object Reference") (OtherActor :type "Actor Object Reference") (OtherComp :type "PrimitiveComponent Object Reference") (OtherBodyIndex :type Integer))
  ; Attack
  (cast `/Game/ThirdPerson/Blueprints/BP_ThirdPersonCharacter` OtherActor)
  (set `self.Attacking` false)
  (goto _label_4 :!via `Close`))

(fn `UserConstructionScript`)